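; An in-world text display that shows production status for the left factory, including its count of produced parts.
; It shows a waiting message on BeginPlay and switches to a production-start message when Start fires.
; UpdateString puts a fixed parts-count caption on the main TextRender and writes the passed-in string to the separate TextDetails component.
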(event `/Game/MyLogic/BPI_StartStop.Start`
  (params (fromLeft :type Boolean))
  (set `self.DefaultString` "Start of production")
  (`TextRenderComponent.K2_SetText` (`self.TextRender`) (`KismetTextLibrary.Conv_StringToText` (`self.DefaultString`)) :!label _label))

(event `self.ReceiveBeginPlay`
  (set `self.DefaultString` "Wait for beginning")
  (goto _label))

(event `/Game/MyLogic/TextRenders/BPI_Text.UpdateString`
  (params (NewString :type String))
  (set `self.DefaultString` "Number of parts produced in the left factory: ")
  (`TextRenderComponent.K2_SetText` (`self.TextRender`) (`KismetTextLibrary.Conv_StringToText` (`self.DefaultString`)))
  (`TextRenderComponent.K2_SetText` (`self.TextDetails`) (`KismetTextLibrary.Conv_StringToText` NewString)))

(fn `UserConstructionScript`)