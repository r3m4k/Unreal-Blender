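; BP_WorkPieceLeft1 is a factory workpiece that travels to a Fabrica machine, gets processed, then moves back toward a manipulator.
; Start waits a delay, then a timeline slides the mesh along Y until Stop halts it and messages Fabrica.
; WorkpieceProcessing animates Z scale to visualize machining, swaps in the completed mesh, signals Fabrica and runs the return timeline.
; StopDetail halts that return move.
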(event `/Game/MyLogic/BPI_StartStop.Start`
  (params (fromLeft :type Boolean))
  (bind (_currentlocation_x _currentlocation_y _currentlocation_z) (`KismetMathLibrary.BreakVector` (`self.CurrentLocation`)))
  (set `self.CurrentLocation` (`SceneComponent.K2_GetComponentLocation` (`self.StaticMesh`)))
  (`KismetSystemLibrary.Delay` (`self.StartDelay`))
  (`KismetSystemLibrary.PrintString` (`self.SelfID`) true true (struct :`R` 1.0 :`G` 0.056582 :`A` 1.0) 3.0)
  (bind (_direction _y_coord) (`Timeline|Y_coord_toFabrica` :`NewTime` 0.0 :!label _label)
    (:`Update`
      (`SceneComponent.K2_SetWorldLocation` (`self.StaticMesh`) (`KismetMathLibrary.MakeVector` _currentlocation_x (+ (* 1000 _y_coord) _currentlocation_y) _currentlocation_z) false false))))

(event `/Game/MyLogic/BPI_StartStop.Stop`
  (message `/Game/MyLogic/BPI_StartStop.Start` (`self.Fabrica`) false)
  (goto _label :!via `Stop`))

(event `/Game/MyLogic/Details/BPI_Details.WorkpieceProcessing`
  (bind (_currentlocation_x _currentlocation_y _currentlocation_z) (`KismetMathLibrary.BreakVector` (`self.CurrentLocation`)))
  (bind (_currentscale_x _currentscale_y _currentscale_z) (`KismetMathLibrary.BreakVector` (`self.CurrentScale`)))
  (set `self.CurrentScale` (`SceneComponent.K2_GetComponentScale` (`self.StaticMesh`)))
  (`KismetSystemLibrary.PrintString` (`self.SelfID`) true true (struct :`R` 0.017893 :`G` 1.0 :`A` 1.0) 3.0)
  ;[1 1 1] Изменим scale по оси Z для визуализации работы станка. При этом по другим осям сохраним значения scale (для этого и создал пременную CurrentScale)
  (bind (_direction _z_scale) (`Timeline|ChangingScale`)
    (:`Update`
      (`SceneComponent.SetRelativeScale3D` (`self.StaticMesh`) (`KismetMathLibrary.MakeVector` _currentscale_x _currentscale_y (* _z_scale _currentscale_z))))
    (:`Finished`
      (`StaticMeshComponent.SetStaticMesh` (`self.StaticMesh`) (`self.CompleteMesh`)) ; Зададим итоговую сетку
      (message `/Game/MyLogic/BPI_StartStop.Stop` (`self.Fabrica`)) ; Остановим манипулятор
      (set `self.CurrentLocation` (`SceneComponent.K2_GetComponentLocation` (`self.StaticMesh`)))
      (bind (_direction_2 _y_coord) (`Timeline|Move_to_Manipulator` :!label _label_2)
        (:`Update`
          (`SceneComponent.K2_SetWorldLocation` (`self.StaticMesh`) (`KismetMathLibrary.MakeVector` _currentlocation_x (+ (* -1000 _y_coord) _currentlocation_y) _currentlocation_z) false false))))))

(event `/Game/MyLogic/Details/BPI_Details.StopDetail`
  (goto _label_2 :!via `Stop`))

(fn `UserConstructionScript`)