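; BP_AssemblyTable is an assembly table that advances a detail mesh through assembly stages, with welding effects.
; Each Start event shows the DetailsMeshes entry at Counter and increments it, with no wrap or bounds check.
; After the first stage, it also messages the welding arm (SvarkaRuka), waits briefly, then activates Niagara sparks.
; The Intencity timeline flickers the point light and deactivates the sparks when it finishes.
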(event `/Game/MyLogic/BPI_StartStop.Start`
  (params (fromLeft :type Boolean))
  (`KismetSystemLibrary.PrintString` "Accembly table is activated" true true (struct :`G` 0.076042 :`B` 1.0 :`A` 1.0) 9.0)
  (`StaticMeshComponent.SetStaticMesh` (`self.DetailMesh`) (`|GetArrayItem` (`self.Details_Meshes`) (`self.Counter`)))
  (if (!= (`self.Counter`) 0)
    (set `self.Counter` (+ (`self.Counter`) 1))
    ;[1 1 1] Запустим анимацию сварочной руки
    (message `/Game/MyLogic/BPI_StartStop.Start` (`self.SvarkaRuka`) false)
    (`KismetSystemLibrary.Delay` 3.5)
    ;[1 1 1] Запустим мерцание источника и искры
    (`ActorComponent.Activate` (`self.Niagara`) false)
    (bind (_direction _intencity) (`Timeline|Intencity`)
      (:`Update`
        (`LightComponent.SetIntensity` (`self.PointLight`) (* 1000 _intencity)))
      (:`Finished`
        (`ActorComponent.Deactivate` (`self.Niagara`))))
    (else
      (set `self.Counter` (+ (`self.Counter`) 1)))))

(fn `UserConstructionScript`)