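; BP_Manipulator is a robotic arm that transfers a part from a left or right conveyor to the assembly table.
; The Transferring event picks a side, then chains timelines that yaw the skeletal mesh to the conveyor, toward the table and finally back, alongside a grab animation and fixed delays.
; The carried part is faked by a side-specific static mesh following a finger socket, hidden before AssemblyTable is messaged.
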(event `/Game/MyLogic/Manipulator/BPI_ManipulatorActions.Transferring `
  (params (fromLeft :type Boolean))
  (bind (_start_angles_x _start_angles_y _start_angles_z) (`KismetMathLibrary.BreakVector` (`self.Start_Angles`)))
  (bind (_start_angles_x_2 _start_angles_y_2 _start_angles_z_2) (`KismetMathLibrary.BreakVector` (`self.Start_Angles`)))
  (bind (_start_angles_x_3 _start_angles_y_3) (`KismetMathLibrary.BreakVector` (`self.Start_Angles`)))
  (`SceneComponent.K2_SetWorldRotation` :`self` (`self.SkeletalMesh`))
  ;[1 1 1] Установим необходимые переменные в зависимости от стороны поворота
  (if fromLeft
    (set `self.isLeft` true)
    (set `self.RotationMultiplier` 1)
    (`KismetSystemLibrary.PrintString` "Take from left" true true (struct :`R` 1.0 :`B` 0.064521 :`A` 1.0) 9.0)
    (bind (_direction _angle) (`Timeline|LeftRotation` :!label _label)
      (:`Update`
        ;[1 1 1] Повернём манипулятор к конвейру с нужной стороны
        (`SceneComponent.K2_SetWorldRotation` (`self.SkeletalMesh`) (`KismetMathLibrary.MakeRotator` _start_angles_x_2 _start_angles_y_2 (+ _start_angles_z_2 (* (`self.RotationMultiplier`) _angle))) false false))
      (:`Finished`
        (`SkeletalMeshComponent.PlayAnimation` (`self.SkeletalMesh`) "/Game/MyLogic/Manipulator/animation1_copy.animation1_copy" false)
        (`KismetSystemLibrary.PrintString` "Animation is activated" true true (struct :`G` 0.66 :`B` 1.0 :`A` 1.0) 9.0)
        (`KismetSystemLibrary.Delay` 4.0)
        (`KismetSystemLibrary.PrintString` "Setting the mesh" true true (struct :`R` 0.190829 :`G` 1.0 :`A` 1.0) 9.0)
        (if (`self.isLeft`)
          (set `self.Index` 0)
          (else
            (set `self.Index` 1)))
        ;[1 1 1] Зададим видимую нужную сетку
        (`StaticMeshComponent.SetStaticMesh` (`self.StaticMesh`) (`|GetArrayItem` (`self.Finger`) (`self.Index`)))
        (`SceneComponent.SetVisibility` (`self.StaticMesh`) true false)
        ;[1 1 1] Повернём манипулятор в нужном направлении во время выполнения анимации для корректной последней точки
        (`KismetSystemLibrary.PrintString` "Rotation to table" true true (struct :`R` 0.203872 :`G` 1.0 :`A` 1.0) 3.0)
        (if (`self.isLeft`)
          (set `self.AddAngle` 0)
          (bind (_direction_2 _angle_2) (`Timeline|Z_Rotation_DuringAnimation` :!label _label_2)
            (:`Update`
              ;[1 1 1] При  этом будем визуально переносить деталь в руке манипулятора
              (`SceneComponent.K2_SetWorldLocation` (`self.StaticMesh`) (`SceneComponent.GetSocketLocation` (`self.SkeletalMesh`) "finger2Socket") false false)
              (`SceneComponent.K2_SetWorldRotation` (`self.SkeletalMesh`) (`KismetMathLibrary.MakeRotator` _start_angles_x_3 _start_angles_y_3 (* (`self.RotationMultiplier`) (+ _angle_2 (`KismetMathLibrary.Conv_IntToDouble` (`self.AddAngle`))))) false false))
            (:`Finished`
              ;[1 1 1] Скроем mesh
              (`KismetSystemLibrary.Delay` 1.5)
              (`SceneComponent.SetVisibility` (`self.StaticMesh`) false false)
              (message `/Game/MyLogic/BPI_StartStop.Start` (`self.AssemblyTable`) false)
              (`KismetSystemLibrary.Delay` 1.5)
              (`KismetSystemLibrary.PrintString` "Setting to start position" true true (struct :`R` 0.106664 :`G` 1.0 :`A` 1.0) 9.0)
              ;[1 1 1] Вернём манипулятор в исходную
              (bind (_direction_3 _angle_3) (`Timeline|Z_Rotation_AfterAnim`)
                (:`Update`
                  (`SceneComponent.K2_SetWorldRotation` (`self.SkeletalMesh`) (`KismetMathLibrary.MakeRotator` _start_angles_x _start_angles_y (+ (+ _angle_3 180.0) _start_angles_z)) false false))
                (:`Finished`
                  (`KismetSystemLibrary.PrintString` "Finish transfering")))))
          (else
            (set `self.AddAngle` 180)
            (goto _label_2)))))
    (else
      (set `self.isLeft` false)
      (set `self.RotationMultiplier` -1)
      (`KismetSystemLibrary.PrintString` "Take from right" true true (struct :`R` 1.0 :`B` 0.064521 :`A` 1.0) 9.0)
      (goto _label))))

(fn `UserConstructionScript`)