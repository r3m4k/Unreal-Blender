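; BP_ApparatSvarkiParent is a parent Blueprint for a welding apparatus at a factory welding table.
; Start plays the apparatus animation once on the skeletal mesh, and Stop halts it.
; Start also sets AddLocation from FromLeft, though both branches assign the same offset.
; A Compensation timeline would shift the mesh along Y from that offset, but nothing triggers it.
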(event `/Game/MyLogic/BPI_StartStop.Start`
  (params (fromLeft :type Boolean))
  (if fromLeft
    (set `self.AddLocation` (100.0 0.0 60.0))
    (else
      (set `self.AddLocation` (100.0 0.0 60.0))))
  (`SkeletalMeshComponent.PlayAnimation` (`self.SkeletalMesh`) "/Game/MyLogic/Fabrica/SvarkaStol/apparatSvarkiAnim.apparatSvarkiAnim" false))

(event `/Game/MyLogic/BPI_StartStop.Stop`
  (`SkeletalMeshComponent.Stop` (`self.SkeletalMesh`)))

(fn `UserConstructionScript`)