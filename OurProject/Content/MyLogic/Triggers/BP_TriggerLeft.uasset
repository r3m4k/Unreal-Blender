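; BP_TriggerLeft is a trigger actor that reacts when anything begins overlapping its box.
; On overlap it prints a debug message, passes true to a Manipulator through TransferringMessage, and calls StopDetailMessage on the current entry of its Details array.
; After a seven-second delay it destroys that detail and increments the counter, so successive triggers work through the array in order.
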(event `self.Box.OnComponentBeginOverlap`
  (params (OverlappedComponent :type "PrimitiveComponent Object Reference") (OtherActor :type "Actor Object Reference") (OtherComp :type "PrimitiveComponent Object Reference") (OtherBodyIndex :type Integer) (bFromSweep :type Boolean) (SweepResult :type "HitResult Structure (by ref)"))
  (bind _output (`|GetArrayItem` (`self.Details`) (`self.Counter`)))
  (`KismetSystemLibrary.PrintString` "Left trigger activated!!!!!!!!!!" true true (struct :`R` 1.0 :`G` 0.027873 :`A` 1.0) 9.0)
  (message `/Game/MyLogic/Manipulator/BPI_ManipulatorActions.Transferring ` (`self.Manipulator`) true)
  (message `/Game/MyLogic/Details/BPI_Details.StopDetail` _output)
  (`KismetSystemLibrary.Delay` 7.0)
  (`self.K2_DestroyActor` _output)
  (set `self.Counter` (+ (`self.Counter`) 1)))

(fn `UserConstructionScript`)