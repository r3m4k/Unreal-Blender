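; BP_TriggerApparatSvarkiLeft is a trigger for the left welding machine that runs workpiece processing when an actor overlaps it.
; On overlap it starts the machine animation on StartTarget, then stops the Workpiece array entry at Counter and plays its processing animation.
; After a fixed delay it sends the processed count to TextRender and increments Counter to select the next workpiece.
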(event `self.ReceiveActorBeginOverlap`
  (params (OtherActor :type "Actor Object Reference"))
  (bind _output (`|GetArrayItem` (`self.Workpiece`) (`self.Counter`)))
  (message `/Game/MyLogic/BPI_StartStop.Start` (`self.StartTarget`) true) ; Запуск анимации обработки
  (message `/Game/MyLogic/BPI_StartStop.Stop` _output) ; Остановка движения заготовки
  (message `/Game/MyLogic/Details/BPI_Details.WorkpieceProcessing` _output) ; Анимация обработки заготовки
  (`KismetSystemLibrary.Delay` 5.0)
  (message `/Game/MyLogic/TextRenders/BPI_Text.UpdateString` (`self.TextRender`) (`KismetStringLibrary.Conv_IntToString` (+ (`self.Counter`) 1)))
  (set `self.Counter` (+ (`self.Counter`) 1)))

(fn `UserConstructionScript`)